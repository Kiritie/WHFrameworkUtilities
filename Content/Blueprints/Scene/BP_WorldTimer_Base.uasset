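; BP_WorldTimer_Base is a base world timer that drives the game's time of day through an Ultra Dynamic Sky actor.
; On initialize it finds the sky if unset and resets timer parameters; lifecycle events start or freeze the clock through TimeSpeed.
; Accessors wrap date, time and day/night lengths, and derive range percentage and an hour-based time phase.
; Time-range wrapping and altitude-based fog logic exist but are never run.
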(event EventOnPreparatory
  (Variables|/UltraDynamicSky/Blueprints/Ultra_Dynamic_Sky.Ultra_Dynamic_Sky_C|SetTime%20Speed (Variables|WorldTimer|GetDynamicSky) 1.0))

(event EventOnInitialize
  (Utilities|IsValid (Variables|WorldTimer|GetDynamicSky)
    (:Is%20Valid
      _)
    (:Is%20Not%20Valid
      (bind _returnvalue (Actor|GetActorOfClass "/UltraDynamicSky/Blueprints/Ultra_Dynamic_Sky.Ultra_Dynamic_Sky_C"))
      (Variables|WorldTimer|SetDynamicSky _returnvalue)))
  (Class|WorldTimer|ResetTimerParams))

(event EventOnRefresh
  (params (DeltaSeconds :type Float%20%28single-precision%29)))

(event EventOnPause
  (Variables|/UltraDynamicSky/Blueprints/Ultra_Dynamic_Sky.Ultra_Dynamic_Sky_C|SetTime%20Speed (Variables|WorldTimer|GetDynamicSky) 0.0))

(event EventOnUnPause
  (Variables|/UltraDynamicSky/Blueprints/Ultra_Dynamic_Sky.Ultra_Dynamic_Sky_C|SetTime%20Speed (Variables|WorldTimer|GetDynamicSky) 1.0))

(fn GetDateTime
  (bind _current_date_and_time (Default|GetCurrentDateandTime (Variables|WorldTimer|GetDynamicSky)))
  (return _current_date_and_time))

(fn SetDateTime
  (params (InDataTime :type Date%20Time%20Structure))
  (Default|SetDateandTime (Variables|WorldTimer|GetDynamicSky) InDataTime))

(fn GetCurrentTime
  (return (Variables|/UltraDynamicSky/Blueprints/Ultra_Dynamic_Sky.Ultra_Dynamic_Sky_C|GetTime%20of%20Day (Variables|WorldTimer|GetDynamicSky))))

(fn SetCurrentTime
  (params (InTime :type Float%20%28single-precision%29))
  (Variables|/UltraDynamicSky/Blueprints/Ultra_Dynamic_Sky.Ultra_Dynamic_Sky_C|SetTime%20of%20Day (Variables|WorldTimer|GetDynamicSky) InTime))

(fn GetSunriseTime
  (return (* 2.4e+03 0.35)))

(fn GetNoonTime
  (return (* 2.4e+03 0.5)))

(fn GetSunsetTime
  (return (* 2.4e+03 0.7)))

(fn GetDayLength
  (return (Variables|/UltraDynamicSky/Blueprints/Ultra_Dynamic_Sky.Ultra_Dynamic_Sky_C|GetDay%20Length (Variables|WorldTimer|GetDynamicSky))))

(fn SetDayLength
  (params (InLength :type Float%20%28single-precision%29))
  (Variables|/UltraDynamicSky/Blueprints/Ultra_Dynamic_Sky.Ultra_Dynamic_Sky_C|SetDay%20Length (Variables|WorldTimer|GetDynamicSky) InLength))

(fn GetNightLength
  (return (Variables|/UltraDynamicSky/Blueprints/Ultra_Dynamic_Sky.Ultra_Dynamic_Sky_C|GetNight%20Length (Variables|WorldTimer|GetDynamicSky))))

(fn SetNightLength
  (params (InLength :type Float%20%28single-precision%29))
  (Variables|/UltraDynamicSky/Blueprints/Ultra_Dynamic_Sky.Ultra_Dynamic_Sky_C|SetNight%20Length (Variables|WorldTimer|GetDynamicSky) InLength))

(fn GetTimeRange
  (return (Variables|WorldTimer|GetMinTime) (Variables|WorldTimer|GetMaxTime)))

(fn GetTimePercent
  (bind (_outmintime _outmaxtime) (CallFunction|GetTimeRange))
  (return (/ (- (CallFunction|GetCurrentTime) _outmintime) (- _outmaxtime _outmintime))))

(fn GetTimePhase
  (bind _returnvalue (CallFunction|GetDateTime))
  (if (< (.hour _returnvalue) 6)
    (return "Night")
    (elif (< (.hour _returnvalue) 8)
      (return "Morning")
      (elif (< (.hour _returnvalue) 11)
        (return "Forenoon")
        (elif (< (.hour _returnvalue) 13)
          (return "Noon")
          (elif (< (.hour _returnvalue) 17)
            (return "Afternoon")
            (elif (< (.hour _returnvalue) 20)
              (return "Evening")
              (else
                (return "Night")))))))))