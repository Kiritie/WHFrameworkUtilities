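; Base world weather Blueprint that wraps Ultra Dynamic Sky and Weather for the game's world framework.
; On init it finds and links both actors, resets to default weather and syncs weather volumes to environment sound events.
; Refresh switches weather around a cloud altitude threshold, pausing freezes weather speed, and weather changes toggle mapped post-process entries.
; Exposes the random seed and random-variation state through get/set parameter functions.
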(event Custom|Weather%20Display%20Name%20Changed_Event
  (params (Weather%20Name :type UDS_Weather_Display_Names%20Enum :default "NewEnumerator0")))

(event Custom|OnWeatherChanged
  (params (Weather%20Name :type UDS_Weather_Display_Names%20Enum :default "NewEnumerator0"))
  (bind _postprocessmapping (Variables|WorldWeather|GetPostProcessMapping))
  (bind _keys (Utilities|Map|Keys _postprocessmapping))
  (for _array_element _keys
    (Variables|/Script/Engine.PostProcessVolume|SetbEnabled (.Value (Utilities|Map|Find _postprocessmapping _array_element)) (Utilities|Enum|Equal(Enum) _array_element Weather%20Name))))

(event Custom|Weather%20Display%20Name%20Changed_Event_0
  (params (Weather%20Name :type UDS_Weather_Display_Names%20Enum :default "NewEnumerator0")))

(event Custom|Weather%20Display%20Name%20Changed_Event_1
  (params (Weather%20Name :type UDS_Weather_Display_Names%20Enum :default "NewEnumerator0")))

(event Custom|Weather%20Display%20Name%20Changed_Event_2
  (params (Weather%20Name :type UDS_Weather_Display_Names%20Enum :default "NewEnumerator0")))

(event Custom|Weather%20Display%20Name%20Changed_Event_3
  (params (Weather%20Name :type UDS_Weather_Display_Names%20Enum :default "NewEnumerator0")))

(event EventOnInitialize
  (Utilities|IsValid (Variables|WorldWeather|GetDynamicSky)
    (:Is%20Valid
      _)
    (:Is%20Not%20Valid
      (bind _returnvalue (Actor|GetActorOfClass "/UltraDynamicSky/Blueprints/Ultra_Dynamic_Sky.Ultra_Dynamic_Sky_C"))
      (Variables|WorldWeather|SetDynamicSky _returnvalue)))
  (Utilities|IsValid (Variables|WorldWeather|GetDynamicWeather)
    (:Is%20Valid
      _)
    (:Is%20Not%20Valid
      (bind _returnvalue_2 (Actor|GetActorOfClass "/UltraDynamicSky/Blueprints/Ultra_Dynamic_Weather.Ultra_Dynamic_Weather_C"))
      (bind _output_get (Variables|WorldWeather|SetDynamicWeather _returnvalue_2))))
  (Default|InitializeWeather _output_get (Variables|WorldWeather|GetDynamicSky))
  (EventDispatchers|AssignWeatherDisplayNameChanged _output_get (EventDispatchers|CreateEvent :!event Custom|OnWeatherChanged))
  (bind _eventdata (|SubscribeEvent self)
    (:then
      (CallFunction|ResetWeatherParams))
    (:Callback
      (if (== (.SoundClass (Utilities|Struct|BreakEventSoundParamsChanged _eventdata)) "/WHFramework/Sounds/Audio/Class/SC_Environment.SC_Environment")
        (Variables|/UltraDynamicSky/Blueprints/Ultra_Dynamic_Weather.Ultra_Dynamic_Weather_C|SetRain%20Volume (Variables|WorldWeather|GetDynamicWeather) (Utilities|Struct|BreakSoundParams (.SoundParams (Utilities|Struct|BreakEventSoundParamsChanged _eventdata))))
        (Variables|/UltraDynamicSky/Blueprints/Ultra_Dynamic_Weather.Ultra_Dynamic_Weather_C|SetClose%20Thunder%20Volume (Variables|WorldWeather|GetDynamicWeather) (Utilities|Struct|BreakSoundParams (.SoundParams (Utilities|Struct|BreakEventSoundParamsChanged _eventdata))))
        (Variables|/UltraDynamicSky/Blueprints/Ultra_Dynamic_Weather.Ultra_Dynamic_Weather_C|SetWind%20Whistling%20Volume (Variables|WorldWeather|GetDynamicWeather) (Utilities|Struct|BreakSoundParams (.SoundParams (Utilities|Struct|BreakEventSoundParamsChanged _eventdata))))
        (Variables|/UltraDynamicSky/Blueprints/Ultra_Dynamic_Weather.Ultra_Dynamic_Weather_C|SetDistant%20Thunder%20Volume (Variables|WorldWeather|GetDynamicWeather) (Utilities|Struct|BreakSoundParams (.SoundParams (Utilities|Struct|BreakEventSoundParamsChanged _eventdata))))
        (Variables|/UltraDynamicSky/Blueprints/Ultra_Dynamic_Weather.Ultra_Dynamic_Weather_C|SetWind%20Volume (Variables|WorldWeather|GetDynamicWeather) (Utilities|Struct|BreakSoundParams (.SoundParams (Utilities|Struct|BreakEventSoundParamsChanged _eventdata))))))))

(event EventOnRefresh
  (params (DeltaSeconds :type Float%20%28single-precision%29))
  (bind _returnvalue (Class|SceneModuleStatics|GetWorldWeather "BP_WorldWeather_Base_C"))
  (bind _cloudaltitude (Variables|WorldWeather|GetCloudAltitude))
  (bind _dynamicweather (Variables|BP_WorldWeather_Base_C|GetDynamicWeather _returnvalue))
  (bind _weather (Variables|/UltraDynamicSky/Blueprints/Ultra_Dynamic_Weather.Ultra_Dynamic_Weather_C|GetWeather _dynamicweather))
  (if (!= _cloudaltitude -1.0)
    (if (< (Class|SceneModuleStatics|GetAltitude (Game|GetPlayerController 0) false) _cloudaltitude)
      (if (== _weather "/UltraDynamicSky/Blueprints/Weather_Effects/Weather_Presets/Clear_Skies.Clear_Skies")
        (Default|ChangeWeather _dynamicweather "/UltraDynamicSky/Blueprints/Weather_Effects/Weather_Presets/Partly_Cloudy.Partly_Cloudy" 0.0))
      (elif (not (== _weather "/UltraDynamicSky/Blueprints/Weather_Effects/Weather_Presets/Clear_Skies.Clear_Skies"))
        (Default|ChangeWeather _dynamicweather "/UltraDynamicSky/Blueprints/Weather_Effects/Weather_Presets/Clear_Skies.Clear_Skies" 0.0)))))

(event EventOnPause
  (Variables|/UltraDynamicSky/Blueprints/Ultra_Dynamic_Weather.Ultra_Dynamic_Weather_C|SetWeather%20Speed (Variables|WorldWeather|GetDynamicWeather) 0.0))

(event EventOnUnPause
  (Variables|/UltraDynamicSky/Blueprints/Ultra_Dynamic_Weather.Ultra_Dynamic_Weather_C|SetWeather%20Speed (Variables|WorldWeather|GetDynamicWeather) 1.0))

(event EventOnPreparatory
  (Variables|/UltraDynamicSky/Blueprints/Ultra_Dynamic_Weather.Ultra_Dynamic_Weather_C|SetWeather%20Speed (Variables|WorldWeather|GetDynamicWeather) 1.0))

(fn SetWeatherParams
  (params (InParams :type Array%20of%20Parameter%20Structures))
  (Default|ApplyState (Variables|/UltraDynamicSky/Blueprints/Ultra_Dynamic_Weather.Ultra_Dynamic_Weather_C|GetRandom_Weather_Variation (Variables|WorldWeather|GetDynamicWeather)) (Utilities|Struct|MakeRandomWeatherVariation_State (.AsUDS%20Weather%20Settings (Utilities|Casting|CastToUDS_Weather_Settings (.Value (|GetParameter (Utilities|Array|Get(acopy) InParams))))) (.Value (|GetParameter (Utilities|Array|Get(acopy) InParams 1))) (.Value (|GetParameter (Utilities|Array|Get(acopy) InParams 2))) (.AsUDS%20Weather%20Settings (Utilities|Casting|CastToUDS_Weather_Settings (.Value (|GetParameter (Utilities|Array|Get(acopy) InParams 3))))))))

(fn GetWeatherParams
  (bind _udw_state (Default|GetStateforSaving (Variables|WorldWeather|GetDynamicWeather)))
  (return (Utilities|Array|MakeArray (|MakeParameter (.TargetRandomWeatherType (Utilities|Struct|BreakRandomWeatherVariation_State (Utilities|Struct|BreakUDS_and_UDW_State _udw_state)))) (|MakeParameter (.CurrentLerpAlpha (Utilities|Struct|BreakRandomWeatherVariation_State (Utilities|Struct|BreakUDS_and_UDW_State _udw_state)))) (|MakeParameter (.CurrentTimerLength (Utilities|Struct|BreakRandomWeatherVariation_State (Utilities|Struct|BreakUDS_and_UDW_State _udw_state)))) (|MakeParameter (.LastRandomWeatherType (Utilities|Struct|BreakRandomWeatherVariation_State (Utilities|Struct|BreakUDS_and_UDW_State _udw_state)))))))

(fn GetWeatherSeed
  (return (Variables|/UltraDynamicSky/Blueprints/Ultra_Dynamic_Weather.Ultra_Dynamic_Weather_C|GetRandom%20Seed (Variables|WorldWeather|GetDynamicWeather))))

(fn SetWeatherSeed
  (params (InSeed :type Integer))
  (Variables|/UltraDynamicSky/Blueprints/Ultra_Dynamic_Weather.Ultra_Dynamic_Weather_C|SetRandom%20Seed (Variables|WorldWeather|GetDynamicWeather) InSeed))

(fn ResetWeatherParams
  (Default|ChangeWeather (Variables|WorldWeather|GetDynamicWeather) (Variables|WorldWeather|GetDefaultWeather) 0.0))