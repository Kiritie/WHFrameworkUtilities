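; BP_WorldWeather is a scene object that wraps an Ultra Dynamic Weather instance for the game world.
; It links the weather to DynamicSky on initialize and zeroes or restores weather speed on pause and unpause.
; Environment sound-class volume changes drive all rain, wind and thunder volumes.
; Getters and setters expose the random seed and random-variation state, packed as generic parameters from the plugin's save state.
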(event Custom|OnSoundParamsChanged
  (params (Sender :type Object%20Object%20Reference) (EventHandle :type Event%20Handle%20Sound%20Params%20Changed%20Object%20Reference))
  (bind _dynamicweather (Variables|WorldWeather|GetDynamicWeather))
  (bind _soundparams (Variables|/Script/WHFramework.EventHandle_SoundParamsChanged|GetSoundParams EventHandle))
  (bind _volume (Utilities|Struct|BreakSoundParams _soundparams))
  (if (== (Variables|/Script/WHFramework.EventHandle_SoundParamsChanged|GetSoundClass EventHandle) "/WHFramework/Audio/Sounds/Class/SC_Environment.SC_Environment")
    (Variables|/UltraDynamicSky/Blueprints/Ultra_Dynamic_Weather.Ultra_Dynamic_Weather_C|SetRain%20Volume _dynamicweather _volume)
    (Variables|/UltraDynamicSky/Blueprints/Ultra_Dynamic_Weather.Ultra_Dynamic_Weather_C|SetClose%20Thunder%20Volume _dynamicweather _volume)
    (Variables|/UltraDynamicSky/Blueprints/Ultra_Dynamic_Weather.Ultra_Dynamic_Weather_C|SetWind%20Whistling%20Volume _dynamicweather _volume)
    (Variables|/UltraDynamicSky/Blueprints/Ultra_Dynamic_Weather.Ultra_Dynamic_Weather_C|SetDistant%20Thunder%20Volume _dynamicweather _volume)
    (Variables|/UltraDynamicSky/Blueprints/Ultra_Dynamic_Weather.Ultra_Dynamic_Weather_C|SetWind%20Volume _dynamicweather _volume)))

(event EventOnInitialize
  (Default|InitializeWeather (Variables|WorldWeather|GetDynamicWeather) (Variables|WorldWeather|GetDynamicSky))
  (Class|EventModuleStatics|SubscribeEvent "/Script/WHFramework.EventHandle_SoundParamsChanged" self "OnSoundParamsChanged"))

(event EventOnRefresh
  (params (DeltaSeconds :type Float%20%28single-precision%29)))

(event EventOnPause
  (Variables|/UltraDynamicSky/Blueprints/Ultra_Dynamic_Weather.Ultra_Dynamic_Weather_C|SetWeather%20Speed (Variables|WorldWeather|GetDynamicWeather) 0.0))

(event EventOnUnPause
  (Variables|/UltraDynamicSky/Blueprints/Ultra_Dynamic_Weather.Ultra_Dynamic_Weather_C|SetWeather%20Speed (Variables|WorldWeather|GetDynamicWeather) 1.0))

(event EventOnPreparatory
  (Variables|/UltraDynamicSky/Blueprints/Ultra_Dynamic_Weather.Ultra_Dynamic_Weather_C|SetWeather%20Speed (Variables|WorldWeather|GetDynamicWeather) 1.0))

(fn SetWeatherParams
  (params (InParams :type Array%20of%20Parameter%20Structures))
  (Default|ApplyState (Variables|/UltraDynamicSky/Blueprints/Ultra_Dynamic_Weather.Ultra_Dynamic_Weather_C|GetRandom_Weather_Variation (Variables|WorldWeather|GetDynamicWeather)) (Utilities|Struct|MakeRandomWeatherVariation_State (Class|ParameterModuleStatics|GetObjectValue (Utilities|Array|Get(acopy) InParams) "/UltraDynamicSky/Blueprints/Weather_Effects/System/UDS_Weather_Settings.UDS_Weather_Settings_C") (Class|ParameterModuleStatics|GetFloatValue (Utilities|Array|Get(acopy) InParams 1)) (Class|ParameterModuleStatics|GetFloatValue (Utilities|Array|Get(acopy) InParams 2)) (Class|ParameterModuleStatics|GetObjectValue (Utilities|Array|Get(acopy) InParams 3) "/UltraDynamicSky/Blueprints/Weather_Effects/System/UDS_Weather_Settings.UDS_Weather_Settings_C"))))

(fn GetWeatherParams
  (bind _udw_state (Default|GetStateforSaving (Variables|WorldWeather|GetDynamicWeather)))
  (return (Utilities|Array|MakeArray (Class|ParameterModuleStatics|MakeObjectParameter (.TargetRandomWeatherType (Utilities|Struct|BreakRandomWeatherVariation_State (Utilities|Struct|BreakUDS_and_UDW_State _udw_state)))) (Class|ParameterModuleStatics|MakeFloatParameter (.CurrentLerpAlpha (Utilities|Struct|BreakRandomWeatherVariation_State (Utilities|Struct|BreakUDS_and_UDW_State _udw_state)))) (Class|ParameterModuleStatics|MakeFloatParameter (.CurrentTimerLength (Utilities|Struct|BreakRandomWeatherVariation_State (Utilities|Struct|BreakUDS_and_UDW_State _udw_state)))) (Class|ParameterModuleStatics|MakeObjectParameter (.LastRandomWeatherType (Utilities|Struct|BreakRandomWeatherVariation_State (Utilities|Struct|BreakUDS_and_UDW_State _udw_state)))))))

(fn GetWeatherSeed
  (return (Variables|/UltraDynamicSky/Blueprints/Ultra_Dynamic_Weather.Ultra_Dynamic_Weather_C|GetRandom%20Seed (Variables|WorldWeather|GetDynamicWeather))))

(fn SetWeatherSeed
  (params (InSeed :type Integer))
  (Variables|/UltraDynamicSky/Blueprints/Ultra_Dynamic_Weather.Ultra_Dynamic_Weather_C|SetRandom%20Seed (Variables|WorldWeather|GetDynamicWeather) InSeed))